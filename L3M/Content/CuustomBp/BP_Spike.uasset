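; BP_Spike is a spike hazard that descends continuously and damages the player.
; BeginPlay enables movement, and Tick lowers the Spikes component along world Z at Speed scaled by delta time, with no stop or reset.
; The DamageZone overlap applies Damage to a BP_FirstPersonCharacter and prints a debug message for any other actor.
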(event OnComponentBeginOverlap(DamageZone)
  (params (OverlappedComponent :type Primitive%20Component%20Object%20Reference) (OtherActor :type Actor%20Object%20Reference) (OtherComp :type Primitive%20Component%20Object%20Reference) (OtherBodyIndex :type Integer) (bFromSweep :type Boolean) (SweepResult :type Hit%20Result%20Structure%20%28by%20ref%29))
  (bind _asbp_first_person_character (Utilities|Casting|CastToBP_FirstPersonCharacter OtherActor)
    (:then
      (Game|Damage|ApplyDamage _asbp_first_person_character (Variables|Default|GetDamage) 0 0))
    (:CastFailed
      (Development|PrintString "This was not player"))))

(event EventTick
  (params (DeltaSeconds :type Float%20%28single-precision%29))
  (bind _spikes (Variables|Default|GetSpikes))
  (bind _returnvalue (Transformation|GetWorldLocation _spikes))
  (if (Variables|Default|GetStartMoving)
    (Transformation|SetWorldLocation _spikes (Math|Vector|MakeVector (.x _returnvalue) (.y _returnvalue) (- (.z _returnvalue) (* (Variables|Default|GetSpeed) DeltaSeconds))) false false)))

(event EventBeginPlay
  (Variables|Default|SetStartMoving true))

(fn ConstructionScript)